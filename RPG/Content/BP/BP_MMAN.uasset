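; Player character Blueprint for a zombie-fighting collection game, won by picking up ten hammer items and lost on death.
; Input drives movement, sprint, jump, montage-timed weapon re-attachment between hand and back, and an alternating two-stage light attack.
; Box overlaps deal random zombie damage, with toggle functions exposed for that hitbox and movement.
; Tick polls the death flag set by damage; both endings share a result-widget macro that enables restarting.
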(event `InputAxis|Turn` :overrideparent false
  (params (AxisValue :type "Float (single-precision)"))
  ;[1 1 1] 滑鼠輸入
  (`self.AddControllerYawInput` AxisValue))

(event `InputAxis|MoveForward` :overrideparent false
  (params (AxisValue :type "Float (single-precision)"))
  ;[1 1 1] 移動
  (if (`self.角色是否死亡`)
    _
    (elif (`self.能否移動`)
      (`self.AddMovementInput` (`KismetMathLibrary.GetForwardVector` (`KismetMathLibrary.MakeRotator` 0.0 0.0 (.yaw (`self.GetControlRotation`)))) AxisValue))))

(event `InputAxis|LookUp` :overrideparent false
  (params (AxisValue :type "Float (single-precision)"))
  ;[1 1 1] 滑鼠輸入
  (`self.AddControllerPitchInput` AxisValue))

(event `InputAction|衝刺`
  (params (Key :type "Key Structure"))
  (bind _charactermovement (`self.CharacterMovement`))
  ;[1 1 1] 控制衝刺
  (:`Pressed`
    (set `CharacterMovementComponent.MaxWalkSpeed` 1000.0 _charactermovement))
  (:`Released`
    (set `CharacterMovementComponent.MaxWalkSpeed` 600.0 _charactermovement)))

(event `InputAxis|MoveRight` :overrideparent false
  (params (AxisValue :type "Float (single-precision)"))
  ;[1 1 1] 移動
  (if (`self.角色是否死亡`)
    _
    (elif (`self.能否移動`)
      (`self.AddMovementInput` (`KismetMathLibrary.GetRightVector` (`KismetMathLibrary.MakeRotator` 0.0 0.0 (.yaw (`self.GetControlRotation`)))) AxisValue))))

(event `InputAction|Jump` :overrideparent false
  (params (Key :type "Key Structure"))
  ;[1 1 1] 跳
  (:`Pressed`
    (if (not (`self.角色是否死亡`))
      (`self.Jump`)))
  (:`Released`
    (`self.StopJumping`)))

(event `InputAction|切換武器`
  (params (Key :type "Key Structure"))
  (bind `_武器` (`self.武器`))
  ;[1 1 1] 切換武器
  (:`Pressed`
    (if (not (`self.角色是否死亡`))
      (set `self.是否拿武器` (not (`self.是否拿武器`)))
      (`|PlayMontage` (`self.Mesh`) "/Game/動畫/切換武器_Montage.切換武器_Montage" ; 播放剪輯動畫
        (:`then`
          (if (`self.是否拿武器`)
            (`KismetSystemLibrary.Delay` 0.8) ; 拿武器延遲
            (`SceneComponent.K2_AttachToComponent` `_武器` (`self.右手掌`) "None" "KeepRelative" "KeepRelative" "KeepRelative" true) ; 有拿武器 手部
            (else
              (`KismetSystemLibrary.Delay` 0.9) ; 放武器延遲
              (`SceneComponent.K2_AttachToComponent` `_武器` (`self.右肩膀`) "None" "KeepRelative" "KeepRelative" "KeepRelative" true) ; 沒拿武器 背部
            ))
          (`KismetSystemLibrary.MoveComponentTo` `_武器`) ; 移動元件到指定位子
        )))))

(event `InputAction|輕攻擊`
  (params (Key :type "Key Structure"))
  (:`Pressed`
    ;[1 1 1] 攻擊
    (if (not (`self.角色是否死亡`))
      (`/Engine/EditorBlueprintResources/StandardMacros.DoOnce` false :!label _label ; 執行一次
        (:`Completed`
          (if (`self.是否拿武器`)
            (`|PlayMontage` (`self.Mesh`) (select `int` (mod (`self.輕攻擊次數`) 2) :`0` "/Game/動畫/輕攻擊第二段_Montage.輕攻擊第二段_Montage" :`1` "/Game/動畫/輕攻擊第一段_Montage.輕攻擊第一段_Montage" :!type "AnimMontage Object Reference") 2.0 ; 播放輕攻擊動畫
              (:`then`
                (`/Engine/EditorBlueprintResources/StandardMacros.IncrementInt` (`self.輕攻擊次數`) ; 遞增 每次加1
                  (:`  `
                    (`KismetSystemLibrary.Delay` 0.6)
                    (`|ExecutionSequence`
                      (:`then_0`
                        (goto _label :!via `Reset`))
                      (:`then_1`
                        (`KismetSystemLibrary.Delay` 0.9)
                        (set `self.輕攻擊次數` 1)))))))
            (else
              (goto _label :!via `Reset`))))))))

(event `self.ReceiveBeginPlay`
  ;[1 1 1] 添加介面
  (bind _returnvalue (`|CreateWidget` "/Game/BP/BW_介面.BW_介面_C" (`GameplayStatics.GetPlayerController` 0)))
  (`UserWidget.AddToViewport` _returnvalue 0))

(event `self.Box.OnComponentBeginOverlap`
  (params (OverlappedComponent :type "PrimitiveComponent Object Reference") (OtherActor :type "Actor Object Reference") (OtherComp :type "PrimitiveComponent Object Reference") (OtherBodyIndex :type Integer) (bFromSweep :type Boolean) (SweepResult :type "HitResult Structure (by ref)"))
  (bind _audio (`self.Audio`))
  ;[1 1 1] 怪物扣血
  (bind `_asbp_殭屍` (cast `/Game/BP/BP_殭屍` OtherActor))
  (`/Game/BP/BP_殭屍.受傷` `_asbp_殭屍` (`KismetMathLibrary.RandomFloatInRange` 1.0 50.0))
  (`AudioComponent.SetSound` _audio "/Game/音效/打.打")
  (`AudioComponent.Play` _audio 0.0))

(event `self.CapsuleComponent.OnComponentBeginOverlap`
  (params (OverlappedComponent :type "PrimitiveComponent Object Reference") (OtherActor :type "Actor Object Reference") (OtherComp :type "PrimitiveComponent Object Reference") (OtherBodyIndex :type Integer) (bFromSweep :type Boolean) (SweepResult :type "HitResult Structure (by ref)"))
  (bind _audio (`self.Audio`))
  ;[1 1 1] 吃道具
  (bind `_asbp_槌子` (cast `/Game/BP/BP_槌子` OtherActor))
  (`AudioComponent.SetSound` _audio "/Game/音效/吃.吃") ; 設定音效
  (`AudioComponent.Play` _audio 0.0) ; 播放
  (`self.K2_DestroyActor` `_asbp_槌子`)
  (bind _result (`/Engine/EditorBlueprintResources/StandardMacros.IncrementInt` (`self.道具數量`))
    (:`  `
      (if (== _result 10)
        (`self.遊戲結束` 0.7 "獲勝")))))

(event `self.ReceiveTick`
  (params (DeltaSeconds :type "Float (single-precision)"))
  ;[1 1 1] 偵測角色死亡
  (if (`self.角色是否死亡`)
    (`/Engine/EditorBlueprintResources/StandardMacros.DoOnce` false ; 執行一次
      (:`Completed`
        (`SkeletalMeshComponent.PlayAnimation` (`self.Mesh`) "/Game/動畫/死亡2.死亡2" false) ; 播放動畫
        (`KismetSystemLibrary.Delay` 2.0) ; 死亡動畫長度
        (`SkeletalMeshComponent.SetPlayRate` (`self.Mesh`) 0.0) ; 動畫定格
        (`self.遊戲結束` 3.0 "失敗")))))

(event `InputAction|重新遊戲`
  (params (Key :type "Key Structure"))
  (:`Pressed`
    (if (`self.是否結束遊戲`)
      (`GameplayStatics.OpenLevel` "NewMap"))))

(fn `UserConstructionScript`)

(fn `切換武器碰撞區域`
  (params (`是否顯示武器碰撞區域` :type Boolean))
  (set `PrimitiveComponent.bGenerateOverlapEvents` `是否顯示武器碰撞區域` (`self.Box`)))

(fn `切換移動`
  (params (`能否移動` :type Boolean))
  (set `self.能否移動` `能否移動`))

(fn `角色受傷`
  (params (`敵人傷害值` :type "Float (double-precision)"))
  (if (`self.是否結束遊戲`)
    _
    (elif (not (`self.角色是否死亡`))
      (set `self.血量` (`KismetMathLibrary.FClamp` (- (`self.血量`) `敵人傷害值`)))
      (`self.PlayAnimMontage` self "/Game/動畫/受傷2_Montage.受傷2_Montage" 1.0 "None")
      (if (<= (`self.血量`) 0.0)
        (set `self.角色是否死亡` true)))))