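; Zombie (殭屍) enemy Blueprint that chases and attacks the BP_MMAN character when it sees it.
; PawnSensing sightings trigger AI MoveTo toward the target unless the attack flag (攻擊玩家) is set.
; Arrival plays a fireball montage through a DoOnce, which resets one second after completion.
; A random wander loop with pauses exists but is disconnected, so it never runs.
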(event `self.ReceiveBeginPlay`
  ;[1 1 1] 隨機移動
)

(event `self.PawnSensing.OnSeePawn`
  (params (Pawn :type "Pawn Object Reference"))
  (if (not (`self.攻擊玩家`))
    (bind _asbp_mman (cast `/Game/BP/BP_MMAN` Pawn))
    (`|AIMoveTo` self (0.0 0.0 0.0) _asbp_mman
      (:`OnSuccess`
        (`/Engine/EditorBlueprintResources/StandardMacros.DoOnce` false :!label _label
          (:`Completed`
            (`|PlayMontage` (`self.Mesh`) "/Game/動畫殭屍/Fireball_Montage.Fireball_Montage"
              (:`then`
                (set `self.攻擊玩家` true))
              (:`OnCompleted`
                (set `self.攻擊玩家` false)
                (`KismetSystemLibrary.Delay` 1.0)
                (goto _label :!via `Reset`)))))))))

(fn `UserConstructionScript`)